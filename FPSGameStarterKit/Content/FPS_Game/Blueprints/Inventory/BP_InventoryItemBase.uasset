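; BP_InventoryItemBase is a base actor for world items the player can store in an inventory.
; On BeginPlay it caches the player's BP_CharacterBase and fills an item struct with itself, class, name and image.
; Sphere overlap toggles the mesh's custom depth and the sphere's Visibility blocking, making it traceable only during overlap.
; StoreThisItem adds the actor to the character's universal inventory, disables sphere collision and hides it instead of destroying it.
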(event `self.ReceiveBeginPlay`
  (bind _asbp_character_base (cast `/Game/FPS_Game/Blueprints/BP_CharacterBase` (`GameplayStatics.GetPlayerCharacter` 0)))
  (set `self.PlayerCast` _asbp_character_base)
  (bind _output_get (set `self.ThisItem` self))
  (set `self.IntentoryDataStruct` (make `/Game/FPS_Game/Blueprints/Inventory/S_InventoryItemStruct` _output_get (`GameplayStatics.GetObjectClass` self) (`self.ItemName`) (`self.ItemImage`))))

(event `self.Sphere.OnComponentBeginOverlap`
  (params (OverlappedComponent :type "PrimitiveComponent Object Reference") (OtherActor :type "Actor Object Reference") (OtherComp :type "PrimitiveComponent Object Reference") (OtherBodyIndex :type Integer) (bFromSweep :type Boolean) (SweepResult :type "HitResult Structure (by ref)"))
  (`PrimitiveComponent.SetRenderCustomDepth` (`self.Mesh`) true)
  (`PrimitiveComponent.SetCollisionResponseToChannel` (`self.Sphere`) "ECC_Visibility" "ECR_Block"))

(event `self.Sphere.OnComponentEndOverlap`
  (params (OverlappedComponent :type "PrimitiveComponent Object Reference") (OtherActor :type "Actor Object Reference") (OtherComp :type "PrimitiveComponent Object Reference") (OtherBodyIndex :type Integer))
  (`PrimitiveComponent.SetRenderCustomDepth` (`self.Mesh`) false)
  (`PrimitiveComponent.SetCollisionResponseToChannel` (`self.Sphere`) "ECC_Visibility" "ECR_Ignore"))

(fn `StoreThisItem`
  (`/Game/FPS_Game/Blueprints/BP_CharacterBase.AddItemToUniversalInventory` (`self.PlayerCast`) (`self.ThisItem`))
  (`PrimitiveComponent.SetCollisionEnabled` (`self.Sphere`) "NoCollision")
  (`self.SetActorHiddenInGame` true))

(fn `UserConstructionScript`)